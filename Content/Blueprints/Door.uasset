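; Door actor that the player toggles open and closed with the Interact input while standing near it.
; Overlap with the Collider by a FirstPersonCharacter enables the door's input, and leaving disables it.
; Each press flips IsDoorClosed and plays or reverses the OpenDoor timeline, which slides the Gate vertically by scaling its Percent track by Height.
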(event OnComponentEndOverlap(Collider)
  (params (OverlappedComponent :type Primitive%20Component%20Object%20Reference) (OtherActor :type Actor%20Object%20Reference) (OtherComp :type Primitive%20Component%20Object%20Reference) (OtherBodyIndex :type Integer))
  (Utilities|Casting|CastToFirstPersonCharacter OtherActor)
  (Input|DisableInput (Game|GetPlayerController 0)))

(event OnComponentBeginOverlap(Collider)
  (params (OverlappedComponent :type Primitive%20Component%20Object%20Reference) (OtherActor :type Actor%20Object%20Reference) (OtherComp :type Primitive%20Component%20Object%20Reference) (OtherBodyIndex :type Integer) (bFromSweep :type Boolean) (SweepResult :type Hit%20Result%20Structure%20%28by%20ref%29))
  (Utilities|Casting|CastToFirstPersonCharacter OtherActor)
  (Input|EnableInput (Game|GetPlayerController 0)))

(event EventBeginPlay)

(event Input|ActionEvents|InputActionInteract
  (params (Key :type Key%20Structure :default "None"))
  (:Pressed
    (if (Variables|Default|GetisDoorClosed)
      (Variables|Default|SetisDoorClosed false)
      (bind _percent (Timeline|OpenDoor Play)
        (:Update
          (Transformation|SetRelativeLocation (Variables|Default|GetGate) (Math|Vector|MakeVector 0.0 0.0 (* _percent (Variables|Default|GetHeight))) false false)))
      (else
        (Variables|Default|SetisDoorClosed true)
        (Timeline|OpenDoor Reverse)))))

(fn ConstructionScript)