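; PressurePlater is a plate-style switch that the first-person character toggles with the Interact input to control other actors.
; Its Collider overlap enables input only while the character is inside, so standing on it alone does not trigger it.
; Each press flips IsOn and sends TurnOn or TurnOff messages to the controlled actors, with TurnOn sent as IsOn becomes false.
; A Timer timeline plays or reverses to sink or raise the Base.
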(event OnComponentEndOverlap(Collider)
  (params (OverlappedComponent :type Primitive%20Component%20Object%20Reference) (OtherActor :type Actor%20Object%20Reference) (OtherComp :type Primitive%20Component%20Object%20Reference) (OtherBodyIndex :type Integer))
  (Utilities|Casting|CastToFirstPersonCharacter OtherActor)
  (Input|DisableInput (Game|GetPlayerController 0)))

(event OnComponentBeginOverlap(Collider)
  (params (OverlappedComponent :type Primitive%20Component%20Object%20Reference) (OtherActor :type Actor%20Object%20Reference) (OtherComp :type Primitive%20Component%20Object%20Reference) (OtherBodyIndex :type Integer) (bFromSweep :type Boolean) (SweepResult :type Hit%20Result%20Structure%20%28by%20ref%29))
  (Utilities|Casting|CastToFirstPersonCharacter OtherActor)
  (Input|EnableInput (Game|GetPlayerController 0)))

(event Input|ActionEvents|InputActionInteract
  (params (Key :type Key%20Structure))
  (bind _otheractorscontrolledbythisactor (Variables|Default|GetOtherActorsControlledByThisActor))
  (:Pressed
    (if (Variables|Default|GetIsOn)
      (Variables|Default|SetIsOn false)
      (Class|ToggleableObject|Turnon(Message) _otheractorscontrolledbythisactor)
      (bind _percent (Timeline|Timer Play)
        (:Update
          (Transformation|SetRelativeLocation (Variables|Default|GetBase) (Math|Vector|MakeVector 0.0 0.0 (* _percent -3.0)) false false)))
      (else
        (Variables|Default|SetIsOn true)
        (Class|ToggleableObject|TurnOff(Message) _otheractorscontrolledbythisactor)
        (Timeline|Timer Reverse)))))

(fn ConstructionScript)