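; ButtonDoor is a double door Blueprint that the player opens and closes with the Interact input while nearby.
; The Collider enables input when a FirstPersonCharacter begins overlapping and disables it when the overlap ends.
; Each press flips IsDoorClosed, prints the action, and plays or reverses the DoorOpen2 timeline, which lerps the yaw of Door1 and Door2 in opposite directions for a 90-degree swing.
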(event OnComponentEndOverlap(Collider)
  (params (OverlappedComponent :type Primitive%20Component%20Object%20Reference) (OtherActor :type Actor%20Object%20Reference) (OtherComp :type Primitive%20Component%20Object%20Reference) (OtherBodyIndex :type Integer))
  (Utilities|Casting|CastToFirstPersonCharacter OtherActor)
  (Input|DisableInput (Game|GetPlayerController 0)))

(event OnComponentBeginOverlap(Collider)
  (params (OverlappedComponent :type Primitive%20Component%20Object%20Reference) (OtherActor :type Actor%20Object%20Reference) (OtherComp :type Primitive%20Component%20Object%20Reference) (OtherBodyIndex :type Integer) (bFromSweep :type Boolean) (SweepResult :type Hit%20Result%20Structure%20%28by%20ref%29))
  (Utilities|Casting|CastToFirstPersonCharacter OtherActor)
  (Input|EnableInput (Game|GetPlayerController 0)))

(event Input|ActionEvents|InputActionInteract
  (params (Key :type Key%20Structure))
  (:Pressed
    (if (Variables|Default|GetisDoorClosed)
      (Development|PrintString "Open")
      (Variables|Default|SetisDoorClosed false)
      (bind _percent (Timeline|DoorOpen2 Play)
        (:Update
          (Transformation|SetRelativeRotation (Variables|Default|GetDoor2) (Math|Rotator|MakeRotator 0.0 0.0 (Math|Float|Lerp 0.0 9e+01 _percent)) false false)
          (Transformation|SetRelativeRotation (Variables|Default|GetDoor1) (Math|Rotator|MakeRotator 0.0 0.0 (Math|Float|Lerp 0.0 -9e+01 _percent)) false false)))
      (else
        (Development|PrintString "Close")
        (Variables|Default|SetisDoorClosed true)
        (Timeline|DoorOpen2 Reverse)))))

(fn ConstructionScript)