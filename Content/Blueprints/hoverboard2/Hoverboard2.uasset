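; Physics-driven hoverboard pawn that the player possesses by interacting, destroying their character, and leaves by spawning a new FirstPersonCharacter.
; The construction script sizes the board and places eight angled arrow thrusters at its corners.
; Each tick, thrusters line trace and push back using a distance falloff curve, while their averaged hit normals drive a self-righting torque toward the ground.
; Input applies forward force, steering torque and camera look.
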(event EventTick
  (params (DeltaSeconds :type Float%20%28single-precision%29))
  ;[1 1 1] Tick
  (CallFunction|ThrustAll DeltaSeconds)
  (CallFunction|ApplyTorque DeltaSeconds))

(event EventPlayerWantstoInteract
  (params (Player :type First%20Person%20Character%20Object%20Reference))
  ;[1 1 1] possess
  (Pawn|Possess (Pawn|GetController Player) self)
  (Actor|DestroyActor Player))

(event Input|ActionEvents|InputActionInteract
  (params (Key :type Key%20Structure :default "None"))
  (bind _root (Variables|Default|GetRoot))
  ;[1 1 1] Unpossess
  (:Pressed
    (bind _returnvalue (Game|SpawnActorfromClass "/Game/Blueprints/PlayerAndGame/FirstPersonCharacter.FirstPersonCharacter_C" (Math|Transform|MakeTransform (+ (Transformation|GetWorldLocation _root) (* (Math|Vector|GetForwardVector _root) 1e+02)) (Math|Rotator|MakeRotator 0.0 0.0 (.yaw (Transformation|GetWorldRotation _root))) "1,1,1") "Undefined" 0 0))
    (Pawn|Possess (Pawn|GetController) _returnvalue)))

(event Input|AxisEvents|InputAxisMoveForward
  (params (AxisValue :type Float%20%28single-precision%29))
  (bind _root (Variables|Default|GetRoot))
  (Physics|AddForce _root (* (Math|Vector|GetForwardVector _root) (* (Variables|Default|GetAcceleration) AxisValue)) "None" true))

(event Input|AxisEvents|InputAxisMoveRight
  (params (AxisValue :type Float%20%28single-precision%29))
  (bind _root (Variables|Default|GetRoot))
  (Class|PrimitiveComponent|AddTorqueinRadians _root (* (Math|Vector|GetUpVector _root) (* AxisValue (Variables|Default|GetSteeringTorque))) "None" true))

(event Input|AxisEvents|InputAxisTurn
  (params (AxisValue :type Float%20%28single-precision%29))
  ;[1 1 1] Mouse look
  (Pawn|Input|AddControllerYawInput AxisValue))

(event Input|AxisEvents|InputAxisLookUp
  (params (AxisValue :type Float%20%28single-precision%29))
  ;[1 1 1] Mouse look
  (Pawn|Input|AddControllerPitchInput AxisValue))

(event Input|AxisEvents|InputAxisTurnRate
  (params (AxisValue :type Float%20%28single-precision%29))
  ;[1 1 1] Stick look
  (Pawn|Input|AddControllerYawInput (* AxisValue 45.0 (Utilities|Time|GetWorldDeltaSeconds))))

(event Input|AxisEvents|InputAxisLookUpRate
  (params (AxisValue :type Float%20%28single-precision%29))
  ;[1 1 1] Stick look
  (Pawn|Input|AddControllerPitchInput (* AxisValue 45.0 (Utilities|Time|GetWorldDeltaSeconds))))

(fn ConstructionScript
  (bind _thruster_height (Variables|Default|GetThruster%20Height))
  (Transformation|SetRelativeScale3D (Variables|Default|GetCube) (Math|Vector|MakeVector (/ (Variables|Default|Getlength) 1e+02) (/ (Variables|Default|Getwidth) 1e+02) 0.1))
  (bind _returnvalue (AddComponent|AddArrowComponent false (Math|Transform|MakeTransform (Math|Vector|MakeVector (/ (Variables|Default|Getlength) 2.0) (/ (Variables|Default|Getwidth) 2.0) _thruster_height) "-45.000000,0.000000, 0" "1,1,1")))
  (bind _returnvalue_2 (AddComponent|AddArrowComponent false (Math|Transform|MakeTransform (Math|Vector|MakeVector (/ (Variables|Default|Getlength) -2.0) (/ (Variables|Default|Getwidth) 2.0) _thruster_height) "-135.000000,0.000000, 0" "1,1,1")))
  (bind _returnvalue_3 (AddComponent|AddArrowComponent false (Math|Transform|MakeTransform (Math|Vector|MakeVector (/ (Variables|Default|Getlength) -2.0) (/ (Variables|Default|Getwidth) -2.0) _thruster_height) "-135.000000,0.000000, 0" "1,1,1")))
  (bind _returnvalue_4 (AddComponent|AddArrowComponent false (Math|Transform|MakeTransform (Math|Vector|MakeVector (/ (Variables|Default|Getlength) 2.0) (/ (Variables|Default|Getwidth) -2.0) _thruster_height) "-45.000000,0.000000, 0" "1,1,1")))
  (bind _returnvalue_5 (AddComponent|AddArrowComponent false (Math|Transform|MakeTransform (Math|Vector|MakeVector (/ (Variables|Default|Getlength) 2.0) (/ (Variables|Default|Getwidth) 2.0) _thruster_height) "-45.000000,90.000000, 0" "1,1,1")))
  (bind _returnvalue_6 (AddComponent|AddArrowComponent false (Math|Transform|MakeTransform (Math|Vector|MakeVector (/ (Variables|Default|Getlength) -2.0) (/ (Variables|Default|Getwidth) 2.0) _thruster_height) "-45.000000,90.000000, 0" "1,1,1")))
  (bind _returnvalue_7 (AddComponent|AddArrowComponent false (Math|Transform|MakeTransform (Math|Vector|MakeVector (/ (Variables|Default|Getlength) -2.0) (/ (Variables|Default|Getwidth) -2.0) _thruster_height) "-135.000000,90.000000, 0" "1,1,1")))
  (bind _returnvalue_8 (AddComponent|AddArrowComponent false (Math|Transform|MakeTransform (Math|Vector|MakeVector (/ (Variables|Default|Getlength) 2.0) (/ (Variables|Default|Getwidth) -2.0) _thruster_height) "-135.000000,90.000000, 0" "1,1,1")))
  (Variables|Default|Setthrusters (Utilities|Array|MakeArray _returnvalue _returnvalue_2 _returnvalue_3 _returnvalue_4 _returnvalue_5 _returnvalue_6 _returnvalue_7 _returnvalue_8)))

(fn Thrustat
  (params (World%20Origin :type Vector) (Dir :type Vector) (Dt :type Float%20%28single-precision%29))
  (bind (_outhit _returnvalue) (Collision|LineTraceByChannel World%20Origin (+ World%20Origin (* Dir (Variables|Default|GetRayLength))) "TraceTypeQuery1" false 0 "ForOneFrame"))
  (if _returnvalue
    (Class|PrimitiveComponent|AddForceatLocation (Variables|Default|GetRoot) (* Dir (* (Math|Curves|GetFloatValue (Variables|Default|GetthrustFalloff) (/ (.Distance (Collision|BreakHitResult _outhit)) (Variables|Default|GetRayLength))) -1.0 (Variables|Default|GetThrust%20Amount) Dt)) World%20Origin "None")
    (Variables|Default|SetGroundNormal (+ (Variables|Default|GetGroundNormal) (.Normal (Collision|BreakHitResult _outhit))))
    (else
      (Variables|Default|SetGroundNormal (+ (Variables|Default|GetGroundNormal) "0, 0,1.000000")))))

(fn ThrustAll
  (params (Dt :type Float%20%28single-precision%29))
  (for _array_element (Variables|Default|Getthrusters)
    (CallFunction|Thrustat (Transformation|GetWorldLocation _array_element) (Math|Vector|GetForwardVector _array_element) Dt)))

(fn ApplyTorque
  (params (Dt :type Float%20%28single-precision%29))
  (bind _root (Variables|Default|GetRoot))
  ;[1 1 1] Average the ground normal
  (Variables|Default|SetGroundNormal (/ (Variables|Default|GetGroundNormal) (Math|Conversions|ToFloat(Integer) (Utilities|Array|Length (Variables|Default|Getthrusters)))))
  (Class|PrimitiveComponent|AddTorqueinRadians _root (* (Math|Vector|CrossProduct (Math|Vector|GetUpVector _root) (Variables|Default|GetGroundNormal)) (* (Variables|Default|Gettorque%20amount) Dt)) "None" true)
  (Variables|Default|SetGroundNormal "0, 0, 0"))