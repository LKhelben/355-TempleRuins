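; MinecartBP is a possessable minecart that builds its own track and lets the player get in, look around and get out.
; Interacting possesses the cart and destroys the player's pawn; pressing Interact again spawns a new FirstPersonCharacter at the camera and possesses it.
; The construction script tiles fixed-length spline meshes along the spline, clamping tangents to piece length.
; No movement along the track is scripted here.
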(event EventPlayerWantstoInteract
  (params (Player :type First%20Person%20Character%20Object%20Reference))
  ;[1 1 1] Get in Cart
  (Pawn|Possess (Pawn|GetController Player) self)
  (Actor|DestroyActor Player))

(event Input|ActionEvents|InputActionInteract
  (params (Key :type Key%20Structure :default "None"))
  (bind _camera (Variables|Default|GetCamera))
  (bind _returnvalue (Transformation|GetWorldTransform _camera))
  (:Pressed
    (bind _returnvalue_2 (Game|SpawnActorfromClass "/Game/Blueprints/FirstPersonCharacter.FirstPersonCharacter_C" (Math|Transform|MakeTransform (.location _returnvalue) (.rotation _returnvalue) "1,1,1") "Undefined" (Components|GetOwner) 0))
    (Pawn|Possess (Pawn|GetController) _returnvalue_2)))

(event Input|AxisEvents|InputAxisTurn
  (params (AxisValue :type Float%20%28single-precision%29))
  ;[1 1 1] Mouse look
  (Pawn|Input|AddControllerYawInput AxisValue))

(event Input|AxisEvents|InputAxisLookUp
  (params (AxisValue :type Float%20%28single-precision%29))
  ;[1 1 1] Mouse look
  (Pawn|Input|AddControllerPitchInput AxisValue))

(event Input|AxisEvents|InputAxisTurnRate
  (params (AxisValue :type Float%20%28single-precision%29))
  ;[1 1 1] Stick look
  (Pawn|Input|AddControllerYawInput (* AxisValue 45.0 (Utilities|Time|GetWorldDeltaSeconds))))

(event Input|AxisEvents|InputAxisLookUpRate
  (params (AxisValue :type Float%20%28single-precision%29))
  ;[1 1 1] Stick look
  (Pawn|Input|AddControllerPitchInput (* AxisValue 45.0 (Utilities|Time|GetWorldDeltaSeconds))))

(fn ConstructionScript
  (bind _spline (Variables|Default|GetSpline))
  (bind _spline_2 (Variables|Default|GetSpline))
  (for _index (range 0 (- (Math|Float|Truncate (/ (Spline|GetSplineLength (Variables|Default|GetSpline)) (Variables|Default|GetLength%20of%20Piece))) 1))
    (bind _returnvalue (AddComponent|AddSplineMeshComponent false))
    (SplineMesh|SetStartandEnd _returnvalue (Spline|GetLocationatDistanceAlongSpline _spline (* _index (Variables|Default|GetLength%20of%20Piece)) "Local") (Math|Vector|ClampVectorSize (Spline|GetTangentatDistanceAlongSpline _spline (* _index (Variables|Default|GetLength%20of%20Piece)) "Local") 0.0 (Variables|Default|GetLength%20of%20Piece)) (Spline|GetLocationatDistanceAlongSpline _spline_2 (* (+ _index 1) (Variables|Default|GetLength%20of%20Piece)) "Local") (Math|Vector|ClampVectorSize (Spline|GetTangentatDistanceAlongSpline _spline_2 (* (+ _index 1) (Variables|Default|GetLength%20of%20Piece)) "Local") 0.0 (Variables|Default|GetLength%20of%20Piece)) true :!class /Script/Engine.SplineMeshComponent)))