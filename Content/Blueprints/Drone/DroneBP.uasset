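; Drone pawn that the player can get into and out of, with mouse and stick look controls.
; PlayerWantstoInteract has the player's controller possess the drone, then calls DestroyActor.
; Pressing Interact spawns a new FirstPersonCharacter just above the drone camera, matching its yaw, and hands possession to it.
; Look input drives controller yaw and pitch, with stick rates scaled by delta time; the graph has no movement input.
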(event EventPlayerWantstoInteract
  (params (Player :type First%20Person%20Character%20Object%20Reference))
  ;[1 1 1] Get in Drone
  (Pawn|Possess (Pawn|GetController Player) self)
  (Actor|DestroyActor))

(event Input|ActionEvents|InputActionInteract
  (params (Key :type Key%20Structure :default "None"))
  (bind _camera (Variables|Default|GetCamera))
  (bind _returnvalue (Transformation|GetWorldTransform _camera))
  ;[1 1 1] Get out of drone
  (:Pressed
    (bind _returnvalue_2 (Game|SpawnActorfromClass "/Game/Blueprints/FirstPersonCharacter.FirstPersonCharacter_C" (Math|Transform|MakeTransform (Math|Vector|MakeVector (.x (.location _returnvalue)) (.y (.location _returnvalue)) (+ (.z (.location _returnvalue)) 2e+01)) (Math|Rotator|MakeRotator 0.0 0.0 (.yaw (.rotation _returnvalue))) "1,1,1") "Undefined" (Components|GetOwner) 0))
    (Pawn|Possess (Pawn|GetController) _returnvalue_2)))

(event Input|AxisEvents|InputAxisTurn
  (params (AxisValue :type Float%20%28single-precision%29))
  ;[1 1 1] Mouse look
  (Pawn|Input|AddControllerYawInput AxisValue))

(event Input|AxisEvents|InputAxisLookUp
  (params (AxisValue :type Float%20%28single-precision%29))
  ;[1 1 1] Mouse look
  (Pawn|Input|AddControllerPitchInput AxisValue))

(event Input|AxisEvents|InputAxisTurnRate
  (params (AxisValue :type Float%20%28single-precision%29))
  ;[1 1 1] Stick look
  (Pawn|Input|AddControllerYawInput (* AxisValue 45.0 (Utilities|Time|GetWorldDeltaSeconds))))

(event Input|AxisEvents|InputAxisLookUpRate
  (params (AxisValue :type Float%20%28single-precision%29))
  ;[1 1 1] Stick look
  (Pawn|Input|AddControllerPitchInput (* AxisValue 45.0 (Utilities|Time|GetWorldDeltaSeconds))))

(fn ConstructionScript)